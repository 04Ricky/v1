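; BP_player is an AR player Blueprint that starts an AR session on BeginPlay and can be moved with the keyboard.
; Every Tick it fetches all tracked AR geometry and debug-draws each element.
; W, A, S and D presses call MovementKeys, which shifts the root by a fixed world-space step without sweep, then increments and prints a move counter.
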(event `self.ReceiveBeginPlay`
  (`ARBlueprintLibrary.StartARSession` "/Game/Blueprints/Ar_sesion_bp.Ar_sesion_bp"))

(event `Key|W`
  (params (Key :type "Key Structure"))
  ;[1 1 1] move keyboard
  (:`Pressed`
    (`self.Movement_keys` (100.0 0.0 0.0))))

(event `Key|S`
  (params (Key :type "Key Structure"))
  ;[1 1 1] move keyboard
  (:`Pressed`
    (`self.Movement_keys` (-100.0 0.0 0.0))))

(event `self.ReceiveTick`
  (params (DeltaSeconds :type "Float (single-precision)"))
  (bind _returnvalue (`ARBlueprintLibrary.GetAllGeometries`))
  (for _array_element _returnvalue
    (`ARBlueprintLibrary.DebugDrawTrackedGeometry` _array_element)))

(event `Key|A`
  (params (Key :type "Key Structure"))
  ;[1 1 1] move keyboard
  (:`Pressed`
    (`self.Movement_keys` (0.0 -100.0 0.0))))

(event `Key|D`
  (params (Key :type "Key Structure"))
  ;[1 1 1] move keyboard
  (:`Pressed`
    (`self.Movement_keys` (0.0 100.0 0.0))))

(fn `Movement_keys`
  (params (DeltaLocation :type "Vector Structure"))
  (`SceneComponent.K2_AddWorldOffset` (`self.DefaultSceneRoot`) DeltaLocation false false)
  (bind _output_get (set `self.Movement_number` (+ (`self.Movement_number`) 1)))
  (`KismetSystemLibrary.PrintString` (`KismetStringLibrary.Conv_IntToString` _output_get)))

(fn `UserConstructionScript`)